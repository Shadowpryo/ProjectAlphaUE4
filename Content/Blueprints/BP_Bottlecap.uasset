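; BP_Bottlecap is a bottle cap projectile that damages basic enemies.
; Each tick it moves along the BottleCap component's forward vector by Speed, without sweeping or scaling by delta time.
; On overlap, if the other actor is the first overlapping BasicEnemy, it applies Strenght as damage and destroys itself.
; Otherwise it destroys itself five seconds after BeginPlay.
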(event EventBeginPlay
  ;[1 1 1] Destorys bottle cap after a few seconds
  (Utilities|FlowControl|Delay 5.0)
  (Actor|DestroyActor))

(event Collision|EventActorBeginOverlap
  (params (OtherActor :type Actor%20Object%20Reference))
  ;[1 1 1] Only desotrys/causes damge if it hits an emey
  (if (== (Utilities|Array|Get(acopy) (Collision|GetOverlappingActors "/Game/Blueprints/BasicEnemy.BasicEnemy_C" :!class /Script/Engine.Actor)) OtherActor)
    (Game|Damage|ApplyDamage OtherActor (Variables|Default|GetStrenght) 0 0)
    (Actor|DestroyActor)))

(event EventTick
  (params (DeltaSeconds :type Float%20%28single-precision%29))
  ;[1 1 1] Moves bottlecap, can change speed
  (Transformation|SetActorLocation (+ (Transformation|GetActorLocation) (* (Math|Vector|GetForwardVector (Variables|Default|GetBottleCap)) (Variables|Default|GetSpeed))) false false))

(fn ConstructionScript)