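; BP_FirstLevel manages a level built around destroying vending machines, handling enemy spawning and the win check.
; On BeginPlay it gathers all BP_VendingMachine actors, stores their count, then makes one capped BasicEnemy spawn attempt.
; The enemy spawns at the player's transform, then moves to an offset from the first machine's mesh.
; CheckForWin takes the remaining machine count, printing a win message at zero or below, otherwise storing it.
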(event Custom|SpawnEnemies
  (bind _vendingm (Variables|Default|GetVendingM))
  (bind _output (Utilities|Array|Get(acopy) _vendingm))
  (bind _staticmesh (Variables|/Game/Blueprints/BP_VendingMachine.BP_VendingMachine_C|GetStaticMesh _output))
  (if (< (Variables|Default|GetCurrentAmountOfEnemies) (Variables|Default|GetMaxEnemiesInWorld))
    (bind _returnvalue (Game|SpawnActorfromClass "/Game/Blueprints/BasicEnemy.BasicEnemy_C" (Transformation|GetActorTransform (Game|GetPlayerCharacter 0)) "Undefined" 0 0))
    (Transformation|SetActorLocation _returnvalue (+ (+ (Math|Vector|GetForwardVector _staticmesh) 5e+01) (Transformation|GetWorldLocation _staticmesh)) false false)))

(event EventBeginPlay
  (bind _outactors (Actor|GetAllActorsOfClass "/Game/Blueprints/BP_VendingMachine.BP_VendingMachine_C"))
  (bind _output_get (Variables|Default|SetVendingM _outactors))
  (Variables|Default|SetVendingsToDestory (Utilities|Array|Length _output_get))
  (CallFunction|SpawnEnemies))

(fn ConstructionScript)

(fn CheckforWin
  (params (NumOfVMs :type Integer))
  (if (<= NumOfVMs 0)
    (Development|PrintString "Level Won")
    (else
      (Variables|Default|SetVendingsToDestory NumOfVMs))))