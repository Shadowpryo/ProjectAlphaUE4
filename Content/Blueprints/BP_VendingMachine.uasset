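; BP_VendingMachine is a damageable level objective that awards score when destroyed and counts toward the win check.
; BeginPlay caches the player and BP_FirstLevel through actor searches.
; AnyDamage subtracts HP, first charging the player's power-up if a BP_Bottlecap comparison passes.
; At zero HP it swaps the mesh for a destructible component, destroys itself after a delay, removes the level list's first entry and updates score.
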(event EventBeginPlay
  ;[1 1 1] Gets refence to player
  (bind _outactors (Actor|GetAllActorsOfClass "/Script/ProjectAlphaUE4.BaseCombatCharacter"))
  (Variables|Default|SetPlayer (Utilities|Array|Get(acopy) _outactors))
  (bind _outactors_2 (Actor|GetAllActorsOfClass "/Game/Blueprints/BP_FirstLevel.BP_FirstLevel_C"))
  (Variables|Default|SetFirstLevel (Utilities|Array|Get(acopy) _outactors_2)))

(event Game|Damage|EventAnyDamage
  (params (Damage :type Float%20%28single-precision%29) (DamageType :type Damage%20Type%20Object%20Reference) (InstigatedBy :type Controller%20Object%20Reference) (DamageCauser :type Actor%20Object%20Reference))
  (bind _firstlevel (Variables|Default|GetFirstLevel))
  (bind _staticmesh (Variables|Default|GetStaticMesh))
  (bind _vendingm (Variables|/Game/Blueprints/BP_FirstLevel.BP_FirstLevel_C|GetVendingM _firstlevel))
  (bind _outactors (Actor|GetAllActorsOfClass "/Game/Blueprints/BP_Bottlecap.BP_Bottlecap_C"))
  (if (== (Utilities|Array|Get(acopy) _outactors) 0)
    (bind _asthird_person_character (Utilities|Casting|CastToThirdPersonCharacter (Variables|Default|GetPlayer)))
    (Default|ChargePowerUp _asthird_person_character))
  (Variables|Default|SetHP (- (Variables|Default|GetHP) Damage))
  (if (<= (Variables|Default|GetHP) 0.0)
    (AddComponent|AddDestructibleComponent false)
    (Rendering|SetVisibility _staticmesh false false)
    (Collision|SetCollisionEnabled _staticmesh "NoCollision")
    (Utilities|FlowControl|Delay 2.0)
    (Actor|DestroyActor)
    (bind _asthird_person_character_2 (Utilities|Casting|CastToThirdPersonCharacter (Variables|Default|GetPlayer)))
    (Utilities|Array|RemoveIndex _vendingm)
    (Default|CheckforWin _firstlevel (Utilities|Array|Length _vendingm))
    (bind _output_get (Variables|/Game/ThirdPersonBP/Blueprints/ThirdPersonCharacter.ThirdPersonCharacter_C|SetScore _asthird_person_character_2 (+ (Variables|/Game/ThirdPersonBP/Blueprints/ThirdPersonCharacter.ThirdPersonCharacter_C|GetScore _asthird_person_character_2) 25)))
    (Default|UpdateScoreText (Variables|/Game/ThirdPersonBP/Blueprints/ThirdPersonCharacter.ThirdPersonCharacter_C|GetScoreUI _asthird_person_character_2) _output_get)))

(fn ConstructionScript)