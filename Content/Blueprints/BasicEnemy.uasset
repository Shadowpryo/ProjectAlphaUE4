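; BasicEnemy is an enemy that turns to face the player every tick and loses HP when it takes damage.
; Hits caused by the first BP_Bottlecap found in the level also charge the player's power-up.
; On death it destroys itself, removes the first entry from the player's EnemiesOnScreen list, adds score and refreshes the score UI, using a player reference cached at BeginPlay.
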(event EventTick
  (params (DeltaSeconds :type Float%20%28single-precision%29))
  ;[1 1 1] Makes enemy face player
  (Transformation|SetWorldRotation (Variables|Collision|GetCapsuleComponent) (Math|Rotator|FindLookatRotation (Transformation|GetActorLocation) (Transformation|GetActorLocation (Game|GetPlayerCharacter 0))) false false))

(event EventBeginPlay
  ;[1 1 1] Gets refence to player
  (bind _outactors (Actor|GetAllActorsOfClass "/Script/ProjectAlphaUE4.BaseCombatCharacter"))
  (Variables|Default|SetPlayer (Utilities|Array|Get(acopy) _outactors)))

(event Game|Damage|EventAnyDamage
  (params (Damage :type Float%20%28single-precision%29) (DamageType :type Damage%20Type%20Object%20Reference) (InstigatedBy :type Controller%20Object%20Reference) (DamageCauser :type Actor%20Object%20Reference))
  ;[1 1 1] Calcualtes damage, kills enemy, charges power up for player
  (bind _outactors (Actor|GetAllActorsOfClass "/Game/Blueprints/BP_Bottlecap.BP_Bottlecap_C"))
  (if (== (Utilities|Array|Get(acopy) _outactors) DamageCauser)
    (bind _asthird_person_character (Utilities|Casting|CastToThirdPersonCharacter (Variables|Default|GetPlayer)))
    (Default|ChargePowerUp _asthird_person_character))
  (Variables|Default|SetHP (- (Variables|Default|GetHP) Damage))
  (if (<= (Variables|Default|GetHP) 0.0)
    (Actor|DestroyActor)
    (bind _asthird_person_character_2 (Utilities|Casting|CastToThirdPersonCharacter (Variables|Default|GetPlayer)))
    (Utilities|Array|RemoveIndex (Variables|/Game/ThirdPersonBP/Blueprints/ThirdPersonCharacter.ThirdPersonCharacter_C|GetEnemiesOnScreen _asthird_person_character_2))
    (bind _output_get (Variables|/Game/ThirdPersonBP/Blueprints/ThirdPersonCharacter.ThirdPersonCharacter_C|SetScore _asthird_person_character_2 (+ (Variables|/Game/ThirdPersonBP/Blueprints/ThirdPersonCharacter.ThirdPersonCharacter_C|GetScore _asthird_person_character_2) 10)))
    (Default|UpdateScoreText (Variables|/Game/ThirdPersonBP/Blueprints/ThirdPersonCharacter.ThirdPersonCharacter_C|GetScoreUI _asthird_person_character_2) _output_get)))

(fn ConstructionScript)